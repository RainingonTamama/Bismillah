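; Rock resource node interactable that swaps between a closed and an open mesh as collection progresses.
; The open mesh shows only while collection is underway; begin play, cancel, depletion and recharge all restore the closed one.
; A disturbance alert plays a sound at the given location and casts player 0 to BP_Killer, but the branch that would show the killer's disturbance indicator is disconnected and never runs.
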(event `self.ReceiveBeginPlay`
  (`SceneComponent.SetVisibility` (`self.MeshComponent`) true false)
  (`SceneComponent.SetVisibility` (`self.Mesh Component Open`) false false))

(event `self.OnCollectionStarted`
  (`SceneComponent.SetVisibility` (`self.MeshComponent`) false false)
  (`SceneComponent.SetVisibility` (`self.Mesh Component Open`) true false))

(event `self.OnCollectionCancelled`
  (`SceneComponent.SetVisibility` (`self.MeshComponent`) true false)
  (`SceneComponent.SetVisibility` (`self.Mesh Component Open`) false false))

(event `self.OnDepleted`
  (`SceneComponent.SetVisibility` (`self.MeshComponent`) true false)
  (`SceneComponent.SetVisibility` (`self.Mesh Component Open`) false false))

(event `self.OnRecharged`
  (`SceneComponent.SetVisibility` (`self.MeshComponent`) true false)
  (`SceneComponent.SetVisibility` (`self.Mesh Component Open`) false false))

(event `self.OnDisturbanceAlert`
  (params (Location :type "Vector Structure"))
  (`GameplayStatics.PlaySoundAtLocation` "/Engine/EditorSounds/GamePreview/EjectFromPlayer_Cue.EjectFromPlayer_Cue" Location (struct) 1.0 1.0 0.0 null null null null)
  (bind _returnvalue (`GameplayStatics.GetPlayerCharacter` 0))
  (bind _asbp_killer (cast `/Game/Characters/BP_Killer` _returnvalue)))

(fn `UserConstructionScript`)